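; Main menu scene Blueprint for Aura that animates a fireball and magic circle decal behind the menu.
; On BeginPlay it records the fireball's start location, plays menu music, shows the main menu widget, and switches to UI-only input with a visible cursor.
; Tick bobs the fireball vertically with a sine of accumulated time, wrapped each full period in UpdateTime, and spins the decal at a configurable rate.
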(event EventBeginPlay
  (bind _returnvalue (Game|GetPlayerController 0))
  (Utilities|FlowControl|Sequence
    (:then_0
      (Variables|Default|SetInitialLocation (Transformation|GetWorldLocation (Variables|Default|GetFireball)))
      (Audio|PlaySound2D "/Game/Assets/Sounds/Music/Music_MainMenu.Music_MainMenu" 1.0 1.0 0.0 0 0))
    (:then_1
      (bind _returnvalue_2 (UserInterface|CreateWidget "/Game/Blueprints/UI/MainMenu/WBP_MainMenu.WBP_MainMenu_C"))
      (UserInterface|Viewport|AddtoViewport _returnvalue_2 0)
      (Input|SetInputModeUIOnly _returnvalue _returnvalue_2 "DoNotLock" false)
      (Variables|/Script/Engine.PlayerController|SetbShowMouseCursor _returnvalue true))))

(event EventTick
  (params (DeltaSeconds :type Float%20%28single-precision%29))
  (bind _initiallocation (Variables|Default|GetInitialLocation))
  (CallFunction|UpdateTime DeltaSeconds)
  (Transformation|SetWorldLocation (Variables|Default|GetFireball) (Math|Vector|MakeVector (.x _initiallocation) (.y _initiallocation) (+ (.z _initiallocation) (* (Math|Trig|Sin(Radians) (Variables|Default|GetTime)) (Variables|Default|GetAmplitude)))) false false)
  (Transformation|AddLocalRotation (Variables|Default|GetMagicCircleDecal) (Math|Rotator|MakeRotator (* (Utilities|Time|GetWorldDeltaSeconds) (Variables|Default|GetMagicCircleRotationRate)) 0.0 0.0) false false))

(fn ConstructionScript)

(fn UpdateTime
  (params (A :type Float%20%28double-precision%29))
  (bind _output_get (Variables|Default|SetTime (+ A (Variables|Default|GetTime))))
  (if (> _output_get (* (Math|Float|MakeLiteralFloat 3.1415) 2.0))
    (Variables|Default|SetTime 0.0)))
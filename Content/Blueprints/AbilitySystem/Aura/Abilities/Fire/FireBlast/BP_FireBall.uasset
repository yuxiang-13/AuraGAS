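; Fireball actor for the Fire Blast ability that flies out, returns to ReturnToActor and explodes near it.
; On the server, an outgoing timeline lerps it to a forward apex, then a returning timeline homes on the actor's current location.
; Within ExplodeDistance it calls OnHit, applies radial damage with upward knockback and death impulse to nearby live players except its owner, then destroys itself.
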(event EventBeginPlay)

(event Collision|EventActorBeginOverlap
  (params (OtherActor :type Actor%20Object%20Reference)))

(event EventTick
  (params (DeltaSeconds :type Float%20%28single-precision%29)))

(event EventStartOutgoingTimeLine
  (bind _returnvalue (Components|GetOwner))
  (bind _explosiondamageparams (Variables|Default|GetExplosionDamageParams))
  (bind _array (Utilities|Array|MakeArray _returnvalue))
  ;[1 1 1] 只控制服务器上的位置移动
  (Networking|SwitchHasAuthority
    (:Authority
      (Variables|Default|SetInitialLocation (Transformation|GetActorLocation))
      (Variables|Default|SetApexLocation (+ (Variables|Default|GetInitialLocation) (* (Transformation|GetActorForwardVector) (Variables|Default|GetTravelDistance))))
      (bind _outgoingtrack (Timeline|OutgoingTimeLine PlayFromStart)
        (:Update
          (Transformation|SetActorLocation (Math|Vector|Lerp(Vector) (Variables|Default|GetInitialLocation) (Variables|Default|GetApexLocation) _outgoingtrack) false false))
        (:Finished
          (bind _新建轨道_0 (Timeline|ReturnningTimeline PlayFromStart)
            (:Update
              (Transformation|SetActorLocation (Math|Vector|Lerp(Vector) (Variables|Default|GetApexLocation) (Transformation|GetActorLocation (Variables|Default|GetReturnToActor)) _新建轨道_0) false false)
              (if (CallFunction|IsWithinExplodeDistance)
                (Class|AuraProjectile|OnHit)
                (Utilities|Array|Add _array self)
                (bind _outoverlappingactors (Class|AuraAbilitySystemLibrary|GetLivePlayerswithinRadius self _array 3e+02 (Transformation|GetActorLocation)))
                (Variables|Default|SetOverlappingPlayers _outoverlappingactors)
                (Class|AuraAbilitySystemLibrary|SetIsRadialDamageEffectParam (Variables|Default|GetExplosionDamageParams) true 5e+01 3e+02 (Transformation|GetActorLocation))
                (for _array_element (Variables|Default|GetOverlappingPlayers)
                  (Class|AuraAbilitySystemLibrary|SetTargetEffectParamsASC (Variables|Default|GetExplosionDamageParams) (Ability|GetAbilitySystemComponent _array_element))
                  (Class|AuraAbilitySystemLibrary|SetKnockbackDirection _explosiondamageparams (Math|Vector|GetForwardVector (Math|Rotator|MakeRotator (.roll (Math|Rotator|MakeRotfromX (- (Transformation|GetActorLocation _array_element) (Transformation|GetActorLocation)))) 45.0 (.yaw (Math|Rotator|MakeRotfromX (- (Transformation|GetActorLocation _array_element) (Transformation|GetActorLocation)))))) 8e+02)
                  (Class|AuraAbilitySystemLibrary|SetDeathImpulseDirection _explosiondamageparams (- (Transformation|GetActorLocation _array_element) (Transformation|GetActorLocation)) 6e+02)
                  (Class|AuraAbilitySystemLibrary|ApplyDamageEffect (Variables|Default|GetExplosionDamageParams)))
                (Actor|DestroyActor)))))))))

(fn ConstructionScript)

(fn IsWithinExplodeDistance
  (return (< (Math|Vector|VectorLength (- (Transformation|GetActorLocation) (Transformation|GetActorLocation (Variables|Default|GetReturnToActor)))) (Variables|Default|GetExplodeDistance))))
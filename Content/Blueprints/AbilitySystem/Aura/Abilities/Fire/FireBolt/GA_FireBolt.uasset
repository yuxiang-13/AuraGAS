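; GA_FireBolt is the Fire Bolt gameplay ability that casts fire projectiles toward the spot or actor under the mouse.
; It commits, reads target data under the cursor, sets the avatar's motion-warp facing through CombatInterface, and plays the cast montage.
; A montage gameplay event triggers SpawnProjectiles from the weapon socket with an overridden launch pitch, homing on the hit actor.
; The ability ends when the montage finishes, blends out or is interrupted.
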(event Ability|EventActivateAbility
  (Ability|CommitAbility)
  (bind _datahandle (|TargetDataUnderMouse)
    (:ValidData
      (Variables|Default|SetProjectileTargetLocation (.Location (Collision|BreakHitResult (Ability|TargetData|GetHitResultfromTargetData _datahandle))))
      (Variables|Default|SetMouse%20Hit%20Actor (.HitActor (Collision|BreakHitResult (Ability|TargetData|GetHitResultfromTargetData _datahandle))))
      ;[1 1 1] 设置运动扭曲参数
      (bind _ascombat_interface (Utilities|Casting|CastToCombatInterface (Ability|GetAvatarActorfromActorInfo)))
      (Class|CombatInterface|UpdateFacingTarget _ascombat_interface (Variables|Default|GetProjectileTargetLocation))
      (|PlayMontageandWaitProxy "None" "/Game/Assets/Characters/Aura/Animations/Abilities/AM_Cast_FireBolt222.AM_Cast_FireBolt222" 1.0 "None" false 1.0 0.0
        (:then
          (Ability|Tasks|WaitGameplayEvent "(TagName=\"Event.Montage.FireBolt\")" 0 true
            (:EventReceived
              (Class|AuraFireBolt|SpawnProjectiles (Variables|Default|GetProjectileTargetLocation) (GameplayTags|MakeLiteralGameplayTag "(TagName=\"CombatSocket_Weapon.Weapon\")") true 45.0 (Variables|Default|GetMouse%20Hit%20Actor)))))
        (:OnCompleted
          (Ability|EndAbility :!label _label))
        (:OnBlendOut
          (goto _label))
        (:OnInterrupted
          (goto _label))
        (:OnCancelled
          (goto _label))))))
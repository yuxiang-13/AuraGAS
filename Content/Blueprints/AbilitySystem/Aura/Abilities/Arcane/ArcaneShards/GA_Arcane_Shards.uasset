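; Arcane Shards gameplay ability that shows a magic circle, then erupts a series of damaging shards around the point clicked under the mouse.
; A spawned BP_PointCollection supplies randomly rotated ground points, while the caster turns and plays a cast montage.
; The montage event hides the circle and starts a looping timer that visits each point, applying radial damage with outward, pitched knockback and firing a GameplayCue.
; After the last point it cleans up and ends.
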(event Custom|SpwnShard
  (if (< (Variables|Default|GetCount) (Variables|Default|GetNum%20Points))
    (CallFunction|StoreShardSpawnLocation)
    (CallFunction|StorePlayerstoDamage)
    (for _array_element (Variables|Default|GetPlayersToDamage)
      (CallFunction|RadialDamagetoPlayer _array_element))
    (Math|Integer|IncrementInt (Variables|Default|GetCount)
      (:%20%20
        ;[1 1 1] 触发Cue
        (Class|GameplayAbility|ExecuteGameplayCuewithParams "(TagName=\"GameplayCue.ArcaneShards\")" (Ability|GameplayCue|MakeGameplayCueParameters :Location (Variables|Default|GetShardSpawnLocation)))))
    (else
      (Utilities|FlowControl|Delay 0.2)
      (Actor|DestroyActor (Variables|Default|GetPointCollection))
      (Utilities|Time|ClearandInvalidateTimerbyHandle (Variables|Default|GetShardSpawnTimer))
      (Ability|EndAbility))))

(event Ability|EventActivateAbility
  (Utilities|FlowControl|Sequence
    (:then_0
      (Class|PlayerInterface|ShowMagicCircle(Message) (Ability|GetAvatarActorfromActorInfo) 0))
    (:then_1
      (Ability|Tasks|WaitInputPress false
        (:OnPress
          (bind _datahandle (|TargetDataUnderMouse) ; 获取鼠标下点位置
            (:ValidData
              (Variables|Default|SetMouseHitLocation (.ImpactPoint (Collision|BreakHitResult (Ability|TargetData|GetHitResultfromTargetData _datahandle))))
              (Utilities|FlowControl|Sequence
                (:then_0
                  (bind _returnvalue (Game|SpawnActorfromClass "/Game/Blueprints/AbilitySystem/Aura/Abilities/Arcane/ArcaneShards/BP_PointCollection.BP_PointCollection_C" (Math|Transform|MakeTransform (Variables|Default|GetMouseHitLocation) "0, 0, 0" "1.000000,1.000000,1.000000") "AlwaysSpawn" "MultiplyWithRoot" 0 0))
                  (bind _output_get (Variables|Default|SetPointCollection _returnvalue))
                  (Variables|Default|SetGroundPoints (Class|PointCollection|GetGroundPoints _output_get (Variables|Default|GetMouseHitLocation) (Variables|Default|GetNum%20Points) (Math|Random|RandomFloatinRange -3.6e+02 3.6e+02))))
                (:then_1
                  (Class|CombatInterface|UpdateFacingTarget(Message) (Ability|GetAvatarActorfromActorInfo) (Variables|Default|GetMouseHitLocation)))
                (:then_2
                  ;[1 1 1] StopWhenAbilityEnd->tue就能保证蒙太奇一定播放
                  (|PlayMontageandWaitProxy "None" "/Game/Assets/Characters/Aura/Animations/Abilities/AM_Cast_ArcaneShards.AM_Cast_ArcaneShards" 1.0 "None" false 1.0 0.0
                    (:then
                      (Ability|Tasks|WaitGameplayEvent "(TagName=\"Event.Montage.ArcaneShards\")" 0 true
                        (:EventReceived
                          ;[1 0 0] 计时器生成第一个魔法阵
                          (bind _returnvalue_2 (Utilities|Time|SetTimerbyEvent (delegate Custom|SpwnShard) (Variables|Default|GetShardSpawnDeltaTime) true))
                          (Variables|Default|SetShardSpawnTimer _returnvalue_2)
                          ;;[1 1 1] 隐藏魔法阵
                          (Class|PlayerInterface|HideMagicCircle(Message) (Ability|GetAvatarActorfromActorInfo) 0)
                          (CallFunction|SpwnShard))))))))))))))

(fn StoreShardSpawnLocation
  (Variables|Default|SetShardSpawnLocation (Transformation|GetWorldLocation (Utilities|Array|Get(acopy) (Variables|Default|GetGroundPoints) (Variables|Default|GetCount))))
  (return))

(fn StorePlayerstoDamage
  (bind _returnvalue (Ability|GetAvatarActorfromActorInfo))
  (bind _outoverlappingactors (Class|AuraAbilitySystemLibrary|GetLivePlayerswithinRadius _returnvalue (Utilities|Array|MakeArray _returnvalue) (Variables|Default|GetRadialDamageOuterRadius) (Variables|Default|GetShardSpawnLocation)))
  (Variables|Default|SetPlayersToDamage _outoverlappingactors))

(fn RadialDamagetoPlayer
  (params (TargetActor :type Actor%20Object%20Reference))
  (bind _returnvalue (Transformation|GetActorLocation TargetActor))
  (bind _shardspawnlocation (Variables|Default|GetShardSpawnLocation))
  (bind _returnvalue_2 (- _returnvalue _shardspawnlocation))
  ;[1 1 1] 应用GE
  (Class|AuraAbilitySystemLibrary|ApplyDamageEffect (Class|AuraDamageGameplayAbility|MakeDamageEffectParamsfromClassDefaults TargetActor (Variables|Default|GetShardSpawnLocation) true _returnvalue_2 true _returnvalue_2 true 35.0)))
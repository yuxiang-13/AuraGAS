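; Electrocute gameplay ability: a channeled lightning beam that shocks the target under the cursor and chains to additional targets.
; A montage event starts looping ShockLoop cues and a timer that commits cost and applies SetByCaller lightning damage.
; Input release (held to a minimum time), failed cost or primary death ends it, applying server-only damage effects and cooldown.
; End cleanup manually resets variables because the ability instance is reused; dead secondary targets drop out individually.
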(event Custom|DamageAndCost
  ;[1 1 1] 消耗和成本
  (bind _returnvalue (Ability|CommitAbilityCost false))
  (if _returnvalue
    (CallFunction|ApplyDamage)
    (else
      (CallFunction|ClearTimerandEndAbility))))

(event Custom|PrepareToEnd
  (bind _mousehitactor (Variables|Default|GetMouseHitActor))
  (Variables|/Script/Engine.PlayerController|SetbShowMouseCursor (Variables|Default|GetOwnerPlayerController) true)
  (Class|CombatInterface|SetinShockLoop(Message) (Ability|GetAvatarActorfromActorInfo) false)
  (Pawn|Components|CharacterMovement|SetMovementMode (Variables|/Script/Engine.Character|GetCharacterMovement (Variables|Default|GetOwnerCharacter)) "MOVE_Walking" 0)
  (if (Variables|Default|GetFirstTargetImplementsInterface)
    (Class|CombatInterface|SetBeingShocked(Message) (Variables|Default|GetMouseHitActor) false)
    (GameplayCue|RemoveGameplayCueOnActor(Looping) _mousehitactor "(TagName=\"GameplayCue.ShockLoop\")" (Variables|Default|GetFirstTargetCueParams))
    (Ability|HasAuthority
      (:True
        ;[1 1 1] 只服务器上应用伤害
        (Class|AuraAbilitySystemLibrary|ApplyDamageEffect (Class|AuraDamageGameplayAbility|MakeDamageEffectParamsfromClassDefaults _mousehitactor)))
      (:False
        _))
    (for _array_element (Variables|Default|GetAdditional%20Targets)
      (Class|CombatInterface|SetBeingShocked(Message) _array_element false)
      (CallFunction|RemoveShockLoopCuefromAdditionalTarget _array_element)
      (Ability|HasAuthority
        (:True
          (Class|AuraAbilitySystemLibrary|ApplyDamageEffect (Class|AuraDamageGameplayAbility|MakeDamageEffectParamsfromClassDefaults _array_element)))))
    (else
      (GameplayCue|RemoveGameplayCueOnActor(Looping) (Ability|GetAvatarActorfromActorInfo) "(TagName=\"GameplayCue.ShockLoop\")" (Variables|Default|GetFirstTargetCueParams)))))

(event Ability|EventActivateAbility
  (if (Utilities|DoesObjectImplementInterface (Ability|GetAvatarActorfromActorInfo) "/Script/Aura.CombatInterface")
    (bind _datahandle (|TargetDataUnderMouse)
      (:ValidData
        (Class|AuraBeamSpell|StoreMouseDataInfo (Ability|TargetData|GetHitResultfromTargetData _datahandle))
        (Class|AuraBeamSpell|StoreOwnerVariables)
        (Utilities|FlowControl|Sequence
          (:then_0
            ;[1 1 1] 隐藏鼠标
            (Variables|/Script/Engine.PlayerController|SetbShowMouseCursor (Variables|Default|GetOwnerPlayerController) false)
            ;[1 1 1] 动作扭曲的朝向
            (Class|CombatInterface|UpdateFacingTarget(Message) (Ability|GetAvatarActorfromActorInfo) (Variables|Default|GetMouseHitLocation))
            (GameplayCue|ExecuteGameplayCue :GameplayCueTag "(TagName=\"GameplayCue.ShockBurst\")")
            (|PlayMontageandWaitProxy "None" (Variables|Default|GetMontage_Electrocute) 1.0 "None" true 1.0 0.0
              (:then
                (Ability|Tasks|WaitGameplayEvent "(TagName=\"Event.Montage.Electrocute\")" 0 true
                  (:EventReceived
                    (Class|CombatInterface|SetinShockLoop(Message) (Ability|GetAvatarActorfromActorInfo) true)
                    (Pawn|Components|CharacterMovement|DisableMovement (Variables|/Script/Engine.Character|GetCharacterMovement (Variables|Default|GetOwnerCharacter)))
                    (Class|AuraBeamSpell|TraceFirstTarget (Variables|Default|GetMouseHitLocation))
                    ;[1 1 1] 生成闪电
                    (CallFunction|SpawnElectricBeam)
                    (bind _returnvalue (Utilities|Time|SetTimerbyEvent (delegate Custom|DamageAndCost) (Variables|Default|GetDamageDeltaTime) true))
                    (Variables|Default|SetDamageAndCostTimer _returnvalue))))))
          (:then_1
            (bind _timeheld (Ability|Tasks|WaitInputRelease false)
              (:OnRelease
                ;[1 1 1] 按键按住的时间
                (bind _output_get (Variables|Default|SetTime%20Held _timeheld))
                (if (< _output_get (Variables|Default|GetMinSpellTime))
                  ;[1 1 1] 只服务器销毁
                  (Ability|HasAuthority
                    (:True
                      (Utilities|FlowControl|Delay (- (Variables|Default|GetMinSpellTime) (Variables|Default|GetTime%20Held)))
                      (CallFunction|ClearTimerandEndAbility :!label _label))
                    (:False
                      ;[1 1 1] 客户端销毁一些展示Cue、鼠标、移动状态
                      (CallFunction|PreparetoEnd)))
                  (else
                    (goto _label)))))))))
    (else
      (Ability|EndAbility))))

(event EventAdditionalTargetDied
  (params (DeadActor :type Actor%20Object%20Reference))
  ;[1 1 1] 次要目标死亡
  (CallFunction|RemoveShockLoopCuefromAdditionalTarget DeadActor)
  (Utilities|Array|RemoveItem (Variables|Default|GetAdditional%20Targets) DeadActor))

(event EventPrimaryTargetDied
  (params (DeadActor :type Actor%20Object%20Reference))
  ;[1 1 1] 主要目标死亡
  ;[1 1 1] 移除Cue
  (GameplayCue|RemoveGameplayCueOnActor(Looping) DeadActor "(TagName=\"GameplayCue.ShockLoop\")" (Variables|Default|GetFirstTargetCueParams))
  ;[1 1 1] 冷却
  (CallFunction|ClearTimerandEndAbility))

(fn SpawnElectricBeam
  (bind _returnvalue (Class|CombatInterface|GetWeapon(Message) (Variables|Default|GetOwnerCharacter)))
  (Variables|Default|SetFirstTargetCueParams (Ability|GameplayCue|MakeGameplayCueParameters :Location (Variables|Default|GetMouseHitLocation) :SourceObject (Variables|Default|GetMouseHitActor) :TargetAttachComponent _returnvalue))
  (bind _output_get (Variables|Default|SetFirstTargetImplementsInterface (Utilities|DoesObjectImplementInterface (Variables|Default|GetMouseHitActor) "/Script/Aura.CombatInterface")))
  (if _output_get
    (LocalVariables|SetCueTarget (Variables|Default|GetMouseHitActor))
    (else
      (LocalVariables|SetCueTarget (Ability|GetAvatarActorfromActorInfo))))
  ;[1 1 1] 创建Cue
  (GameplayCue|AddGameplayCueOnActor(Looping) (LocalVariables|GetCueTarget) "(TagName=\"GameplayCue.ShockLoop\")" (Variables|Default|GetFirstTargetCueParams))
  (if (Variables|Default|GetFirstTargetImplementsInterface)
    (Class|CombatInterface|SetBeingShocked(Message) (LocalVariables|GetCueTarget) true)
    (bind _outadditionaltargets (Class|AuraBeamSpell|StoreAdditionalTargets))
    (bind _output_get_2 (Variables|Default|SetAdditional%20Targets _outadditionaltargets))
    (for _array_element _output_get_2
      (Class|CombatInterface|SetBeingShocked(Message) _array_element true)
      (CallFunction|AddShockLoopCuetoAdditionalTarget _array_element))))

(fn AddShockLoopCuetoAdditionalTarget
  (params (AdditionalTarget :type Actor%20Object%20Reference))
  (LocalVariables|SetTargetActor AdditionalTarget)
  (Utilities|Map|Add (Variables|Default|GetAdditionActorsToCue) (LocalVariables|GetTargetActor) (Ability|GameplayCue|MakeGameplayCueParameters :Location (Transformation|GetActorLocation (LocalVariables|GetTargetActor)) :SourceObject (LocalVariables|GetTargetActor) :TargetAttachComponent (Variables|/Script/Engine.Actor|GetRootComponent (Variables|Default|GetMouseHitActor))))
  (GameplayCue|AddGameplayCueOnActor(Looping) (LocalVariables|GetTargetActor) "(TagName=\"GameplayCue.ShockLoop\")" (Ability|GameplayCue|MakeGameplayCueParameters :Location (Transformation|GetActorLocation (LocalVariables|GetTargetActor)) :SourceObject (LocalVariables|GetTargetActor) :TargetAttachComponent (Variables|/Script/Engine.Actor|GetRootComponent (Variables|Default|GetMouseHitActor)))))

(fn RemoveShockLoopCuefromAdditionalTarget
  (params (AdditionalTarget :type Actor%20Object%20Reference))
  (LocalVariables|SetTarget AdditionalTarget)
  (if (.ReturnValue (Utilities|Map|Find (Variables|Default|GetAdditionActorsToCue) (LocalVariables|GetTarget)))
    (GameplayCue|RemoveGameplayCueOnActor(Looping) (LocalVariables|GetTarget) "(TagName=\"GameplayCue.ShockLoop\")" (.Value (Utilities|Map|Find (Variables|Default|GetAdditionActorsToCue) (LocalVariables|GetTarget))))))

(fn ApplyDamage
  (CallFunction|ApplyDamageSingleTarget (Variables|Default|GetMouseHitActor))
  (for _array_element (Variables|Default|GetAdditional%20Targets)
    (CallFunction|ApplyDamageSingleTarget _array_element)))

(fn ApplyDamageSingleTarget
  (params (Actor :type Actor%20Object%20Reference))
  (bind _output_get (LocalVariables|SetTargetASC (Ability|GetAbilitySystemComponent Actor)))
  (Utilities|IsValid _output_get
    (:Is%20Valid
      (bind _output_get_2 (LocalVariables|SetASC (Ability|GetAbilitySystemComponentfromActorInfo)))
      (Utilities|IsValid _output_get_2
        (:Is%20Valid
          ;[1 1 1] 分配设置伤害数值修改（SetByCaller）
          (bind _returnvalue (Ability|GameplayEffect|AssignTagSetbyCallerMagnitude (GameplayEffects|MakeOutgoingSpec (LocalVariables|GetASC) (Variables|Default|GetDamageEffectClass) (Math|Conversions|ToFloat(Integer) (Ability|GetAbilityLevel)) (GameplayEffects|MakeEffectContext (LocalVariables|GetASC))) "(TagName=\"Damage.Lightning\")" (Class|AuraDamageGameplayAbility|GetDamageatLevel)))
          (GameplayEffects|ApplyGameplayEffectSpecToSelf (LocalVariables|GetTargetASC) _returnvalue))))))

(fn ClearTimerandEndAbility
  (Utilities|Time|ClearandInvalidateTimerbyHandle (Variables|Default|GetDamageAndCostTimer))
  (CallFunction|PreparetoEnd)
  (Ability|CommitAbilityCooldown false)
  ;[1 1 1] 因为每个GA都自己只实例化1个！所以要结束GA前，清空重置一些参数
  (Utilities|Array|Clear (Variables|Default|GetAdditional%20Targets))
  (Utilities|Map|Clear (Variables|Default|GetAdditionActorsToCue))
  (Variables|Default|SetMouseHitActor 0)
  (Variables|Default|SetFirstTargetImplementsInterface false)
  (Variables|Default|SetTime%20Held 0.0)
  (Ability|EndAbility))